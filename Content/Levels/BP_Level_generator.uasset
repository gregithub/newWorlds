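; Procedural level generator that builds a random grid of connected room actors on BeginPlay.
; A random walk from the grid centre places rooms, backtracking at dead ends or by branch chance.
; Connection flags are mirrored between neighbours, and extra random links join adjacent rooms.
; It spawns room Blueprints only for one-connection (rotated to fit) and four-connection (randomly rotated) cells, then issues RebuildNavigation.
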(event `self.ReceiveBeginPlay`
  (`self.GenerateLevel` (-4000.0 -4000.0 0.0) (9.0 9.0) (1000.0 1000.0) 16 0.2 2 3))

(event `GenerateLevel`
  (params (Starting_Position :type "Vector Structure") (Level_Dimensions :type "Vector2D Structure") (Room_Dimensions :type "Vector2D Structure") (Number_Of_Rooms :type Integer) (Branch_Chance :type "Float (double-precision)") (Extra_Connections :type Integer) (Max_Branch_Length :type Integer))
  (bind _current_room (`self.Current_Room`))
  (bind _current_room_2 (`self.Current_Room`))
  (bind _level_dimensions_x (`self.Level_Dimensions_X`))
  (bind _rooms (`self.Rooms`))
  (bind _current_room_3 (`self.Current_Room`))
  (bind _movement_direrctions (`self.Movement_Direrctions`))
  (bind _current_room_4 (`self.Current_Room`))
  (bind _level_dimensions_x_2 (`self.Level_Dimensions_X`))
  (bind _movement_direrctions_2 (`self.Movement_Direrctions`))
  (bind _current_room_5 (`self.Current_Room`))
  (bind _level_dimensions_x_3 (`self.Level_Dimensions_X`))
  (bind _movement_direrctions_3 (`self.Movement_Direrctions`))
  (bind _current_room_6 (`self.Current_Room`))
  (bind _level_dimensions_x_4 (`self.Level_Dimensions_X`))
  (bind _movement_direrctions_4 (`self.Movement_Direrctions`))
  (bind _room_placed (`self.Room Placed`))
  (bind _current_room_7 (`self.Current_Room`))
  (bind _level_dimensions_x_5 (`self.Level_Dimensions_X`))
  (bind _connected_rooms (`self.Connected_Rooms`))
  (bind _room_placed_2 (`self.Room Placed`))
  (bind _current_room_8 (`self.Current_Room`))
  (bind _movement_direrctions_5 (`self.Movement_Direrctions`))
  (bind _current_room_9 (`self.Current_Room`))
  (bind _level_dimensions_x_6 (`self.Level_Dimensions_X`))
  (bind _level_dimensions_x_7 (`self.Level_Dimensions_X`))
  (bind _current_room_10 (`self.Current_Room`))
  (bind _level_dimensions_x_8 (`self.Level_Dimensions_X`))
  (bind (_x _y) (`KismetMathLibrary.BreakVector2D` (`self.Level_Dimensions`)))
  (bind _returnvalue (- _current_room_2 (`self.Previous_Room`)))
  (bind _returnvalue_2 (- (`self.Main_Loop_Index`) 1))
  (bind _returnvalue_3 (- (`self.Main_Loop_Index`) (`self.Level_Dimensions_X`)))
  (bind (_x_2 _y_2) (`KismetMathLibrary.BreakVector2D` (`self.Room_Dimensions`)))
  (bind (_x_3 _y_3) (`KismetMathLibrary.BreakVector2D` (`self.Level_Dimensions`)))
  (bind _returnvalue_4 (* (`self.Level_Dimensions_X`) (`self.Level_Dimensions_Y`)))
  (bind _returnvalue_5 (+ (`self.Main_Loop_Index`) 1))
  (bind _returnvalue_6 (+ (`self.Main_Loop_Index`) (`self.Level_Dimensions_X`)))
  (bind (_left _right _up _down) (break `/Game/Levels/STRUCT_Connected_Rooms` (`|GetArrayItem` (`self.Connected_Rooms`) (`self.Main_Loop_Index`))))
  (bind (_left_2 _right_2 _up_2 _down_2) (break `/Game/Levels/STRUCT_Connected_Rooms` (`|GetArrayItem` (`self.Connected_Rooms`) (`self.Current_Room`))))
  (bind (_left_3 _right_3 _up_3 _down_3) (break `/Game/Levels/STRUCT_Connected_Rooms` (`|GetArrayItem` (`self.Connected_Rooms`) (`self.Previous_Room`))))
  (bind (_left_4 _right_4 _up_4 _down_4) (break `/Game/Levels/STRUCT_Connected_Rooms` (`|GetArrayItem` (`self.Connected_Rooms`) (`self.Current_Room`))))
  (bind (_left_5 _right_5 _up_5 _down_5) (break `/Game/Levels/STRUCT_Connected_Rooms` (`|GetArrayItem` (`self.Connected_Rooms`) (`self.Main_Loop_Index`))))
  (bind (_left_6 _right_6 _up_6 _down_6) (break `/Game/Levels/STRUCT_Connected_Rooms` (`|GetArrayItem` (`self.Connected_Rooms`) (`self.Main_Loop_Index`))))
  (bind (_left_7 _right_7 _up_7 _down_7) (break `/Game/Levels/STRUCT_Connected_Rooms` (`|GetArrayItem` (`self.Connected_Rooms`) _returnvalue_5)))
  (bind (_left_8 _right_8 _up_8 _down_8) (break `/Game/Levels/STRUCT_Connected_Rooms` (`|GetArrayItem` (`self.Connected_Rooms`) _returnvalue_2)))
  (bind (_left_9 _right_9 _up_9) (break `/Game/Levels/STRUCT_Connected_Rooms` (`|GetArrayItem` (`self.Connected_Rooms`) _returnvalue_3)))
  (bind (_left_10 _right_10 _up_10 _down_9) (break `/Game/Levels/STRUCT_Connected_Rooms` (`|GetArrayItem` (`self.Connected_Rooms`) _returnvalue_6)))
  ;[1 0.5204 0.5403] Setting variables
  (set `self.Starting_Position` Starting_Position)
  (set `self.Level_Dimensions` Level_Dimensions)
  (set `self.Room_Dimensions` Room_Dimensions)
  (set `self.Number_Of_Rooms` Number_Of_Rooms)
  (set `self.Branch_Chance` Branch_Chance)
  (set `self.Extra_Connections` Extra_Connections)
  (set `self.Max_Branch_Length` Max_Branch_Length)
  (set `self.Previous_Room` -1)
  (`KismetArrayLibrary.Array_Clear` (`self.Steps_Taken`))
  (set `self.Level_Dimensions_X` (`KismetMathLibrary.FFloor` _x))
  (set `self.Level_Dimensions_Y` (`KismetMathLibrary.FFloor` _y))
  (for _array_element _rooms
    (`self.K2_DestroyActor` _array_element))
  (`KismetArrayLibrary.Array_Clear` _rooms)
  (`KismetArrayLibrary.Array_Resize` _rooms _returnvalue_4)
  (`KismetArrayLibrary.Array_Clear` _room_placed)
  (`KismetArrayLibrary.Array_Resize` _room_placed _returnvalue_4)
  (`KismetArrayLibrary.Array_Clear` _connected_rooms)
  (`KismetArrayLibrary.Array_Resize` _connected_rooms _returnvalue_4)
  (set `self.Current_Room` (+ (`KismetMathLibrary.FFloor` (* _x_3 0.5)) (* (`KismetMathLibrary.FFloor` (* _y_3 0.5)) (`self.Level_Dimensions_X`))))
  (for _index (range 1 (+ (`self.Number_Of_Rooms`) 1))
    (set `self.Main_Loop_Index` _index)
    ;[1 1 1] Allocate room
    (`KismetArrayLibrary.Array_Add` (`self.Steps_Taken`) _current_room)
    (`KismetArrayLibrary.Array_Set` (`self.Room Placed`) _current_room true)
    ;[1 1 1] If this is the first room
    (if (not (== (`self.Previous_Room`) -1))
      ;[1 1 1] Inform About Connected Room(FIrst Stage)
      (`KismetArrayLibrary.Array_Set` (`self.Connected_Rooms`) _current_room_2 (make `/Game/Levels/STRUCT_Connected_Rooms` (== _returnvalue 1) (== _returnvalue -1) (== _returnvalue _level_dimensions_x) (== _returnvalue (* _level_dimensions_x -1))))
      ;[1 1 1] Check if map is full
      (if (< (`KismetArrayLibrary.Array_Length` (`self.Steps_Taken`)) (* (`self.Level_Dimensions_X`) (`self.Level_Dimensions_Y`)))
        ;[1 1 1] Random Chance to Step Back
        (if (not (> (`KismetMathLibrary.RandomFloat`) (`self.Branch_Chance`)))
          (set `self.Main_Loop_Index` (`KismetMathLibrary.Max` (- (`self.Main_Loop_Index`) (`KismetMathLibrary.RandomIntegerInRange` 1 (`self.Max_Branch_Length`)))))
          (set `self.Current_Room` (`|GetArrayItem` (`self.Steps_Taken`) (`self.Main_Loop_Index`))))
        (else
          (break))))
    (`|ExecutionSequence` :!label _label
      (:`then_0`
        ;[1 1 1] Left
        (if (> (mod _current_room_3 (`self.Level_Dimensions_X`)) 0)
          (if (`|GetArrayItem` (`self.Room Placed`) (- _current_room_3 1))
            (`KismetArrayLibrary.Array_Add` _movement_direrctions :!label _label_2)
            (else
              (`KismetArrayLibrary.Array_Add` _movement_direrctions true)))
          (else
            (goto _label_2))))
      (:`then_1`
        ;[1 1 1] Right
        (if (< (mod _current_room_4 _level_dimensions_x_2) (- _level_dimensions_x_2 1))
          (if (`|GetArrayItem` (`self.Room Placed`) (+ _current_room_4 1))
            (`KismetArrayLibrary.Array_Add` _movement_direrctions_2 :!label _label_3)
            (else
              (`KismetArrayLibrary.Array_Add` _movement_direrctions_2 true)))
          (else
            (goto _label_3))))
      (:`then_2`
        ;[1 1 1] UP
        (if (>= _current_room_5 _level_dimensions_x_3)
          (if (`|GetArrayItem` (`self.Room Placed`) (- _current_room_5 _level_dimensions_x_3))
            (`KismetArrayLibrary.Array_Add` _movement_direrctions_3 :!label _label_4)
            (else
              (`KismetArrayLibrary.Array_Add` _movement_direrctions_3 true)))
          (else
            (goto _label_4))))
      (:`then_3`
        ;[1 1 1] DOWN
        (if (< _current_room_6 (* _level_dimensions_x_4 (- (`self.Level_Dimensions_Y`) 1)))
          (if (`|GetArrayItem` (`self.Room Placed`) (+ _current_room_6 _level_dimensions_x_4))
            (`KismetArrayLibrary.Array_Add` _movement_direrctions_4 :!label _label_5)
            (else
              (`KismetArrayLibrary.Array_Add` _movement_direrctions_4 true)))
          (else
            (goto _label_5))))
      (:`then_4`
        ;[1 1 1] Count Number Of Move Options
        (`self.Check Move Options`
          (:`Choose`
            ;[1 1 1] CHoose random direction to move
            (set `self.Move_Choice` (`KismetMathLibrary.RandomIntegerInRange` 1 (`self.Move_Options`)))
            (for (_array_element_2 _array_index) (`self.Movement_Direrctions`)
              (if _array_element_2
                (set `self.Movement_Direction_Search` (+ (`self.Movement_Direction_Search`) 1))
                (if (== (`self.Move_Choice`) (`self.Movement_Direction_Search`))
                  (set `self.Previous_Room` (`self.Current_Room`))
                  (set `self.Current_Room` (select `int` _array_index :`0` (- _current_room_7 1) :`1` (+ _current_room_7 1) :`2` (- _current_room_7 _level_dimensions_x_5) :`3` (+ _current_room_7 _level_dimensions_x_5)))
                  ;[1 1 1] Clear Variables
                  (`KismetArrayLibrary.Array_Clear` (`self.Movement_Direrctions`) :!label _label_6)
                  (set `self.Move_Options` 0)
                  (set `self.Movement_Direction_Search` 0)))))
          (:`Try Again`
            (set `self.Main_Loop_Index` (- (`self.Main_Loop_Index`) 1))
            (set `self.Current_Room` (`|GetArrayItem` (`self.Steps_Taken`) (`self.Main_Loop_Index`)))
            ;[1 1 1] Reset before break
            (`KismetArrayLibrary.Array_Clear` (`self.Movement_Direrctions`))
            (set `self.Move_Options` 0)
            (goto _label))))))
  (`|ExecutionSequence`
    (:`then_0`
      ;[1 1 1] Inform about connected room(Second stage)
      (for _array_element_3 (`self.Steps_Taken`)
        (set `self.Main_Loop_Index` _array_element_3)
        (`|ExecutionSequence`
          (:`then_0`
            (if _left
              (`KismetArrayLibrary.Array_Set` (`self.Connected_Rooms`) _returnvalue_2 (make `/Game/Levels/STRUCT_Connected_Rooms` _left_8 true _up_8 _down_8))))
          (:`then_1`
            (if _right
              (`KismetArrayLibrary.Array_Set` (`self.Connected_Rooms`) _returnvalue_5 (make `/Game/Levels/STRUCT_Connected_Rooms` true _right_7 _up_7 _down_7))))
          (:`then_2`
            (if _up
              (`KismetArrayLibrary.Array_Set` (`self.Connected_Rooms`) _returnvalue_3 (make `/Game/Levels/STRUCT_Connected_Rooms` _left_9 _right_9 _up_9 true))))
          (:`then_3`
            (if _down
              (`KismetArrayLibrary.Array_Set` (`self.Connected_Rooms`) _returnvalue_6 (make `/Game/Levels/STRUCT_Connected_Rooms` _left_10 _right_10 true _down_9)))))))
    (:`then_1`
      ;[1 1 1] Randomly Connect Rooms Together
      (for _ (range 1 (+ (`self.Extra_Connections`) 1))
        (set `self.Extra_Connectrions_Attempts` 0)
        (set `self.Current_Room` (`|GetArrayItem` (`self.Steps_Taken`) (`KismetMathLibrary.RandomInteger` (`self.Number_Of_Rooms`))) :!label _label_7)
        (set `self.Extra_Connectrions_Attempts` (+ (`self.Extra_Connectrions_Attempts`) 1))
        (`|ExecutionSequence`
          (:`then_0`
            (if (> (mod _current_room_9 _level_dimensions_x_6) 0)
              (if _left_2
                (`KismetArrayLibrary.Array_Add` (`self.Movement_Direrctions`) :!label _label_8)
                (else
                  (`KismetArrayLibrary.Array_Add` _movement_direrctions_5 (`|GetArrayItem` _room_placed_2 (- _current_room_8 1)))))
              (else
                (goto _label_8))))
          (:`then_1`
            (if (< (mod _current_room_9 _level_dimensions_x_6) (- _level_dimensions_x_6 1))
              (if _right_2
                (goto _label_8)
                (else
                  (`KismetArrayLibrary.Array_Add` _movement_direrctions_5 (`|GetArrayItem` _room_placed_2 (+ _current_room_8 1)))))
              (else
                (goto _label_8))))
          (:`then_2`
            (if (>= _current_room_9 _level_dimensions_x_6)
              (if _up_2
                (goto _label_8)
                (else
                  (`KismetArrayLibrary.Array_Add` _movement_direrctions_5 (`|GetArrayItem` _room_placed_2 (- _current_room_8 _level_dimensions_x_7)))))
              (else
                (goto _label_8))))
          (:`then_3`
            (if (< _current_room_9 (* _level_dimensions_x_6 (- (`self.Level_Dimensions_Y`) 1)))
              (if _down_2
                (goto _label_8)
                (else
                  (`KismetArrayLibrary.Array_Add` _movement_direrctions_5 (`|GetArrayItem` _room_placed_2 (+ _current_room_8 _level_dimensions_x_7)))))
              (else
                (goto _label_8))))
          (:`then_4`
            (`self.Check Move Options`
              (:`Choose`
                (set `self.Move_Choice` (`KismetMathLibrary.RandomIntegerInRange` 1 (`self.Move_Options`)))
                (for (_array_element_4 _array_index_2) (`self.Movement_Direrctions`)
                  (if _array_element_4
                    (set `self.Main_Loop_Index` _array_index_2)
                    (set `self.Movement_Direction_Search` (+ (`self.Movement_Direction_Search`) 1))
                    (if (== (`self.Movement_Direction_Search`) (`self.Move_Choice`))
                      (set `self.Previous_Room` (select `int` (`self.Main_Loop_Index`) :`0` (- _current_room_10 1) :`1` (+ _current_room_10 1) :`2` (- _current_room_10 _level_dimensions_x_8) :`3` (+ _current_room_10 _level_dimensions_x_8)))
                      (`KismetArrayLibrary.Array_Set` (`self.Connected_Rooms`) (`self.Current_Room`) (select `int` (`self.Main_Loop_Index`) :`0` (make `/Game/Levels/STRUCT_Connected_Rooms` true _right_4 _up_4 _down_4) :`1` (make `/Game/Levels/STRUCT_Connected_Rooms` _left_4 true _up_4 _down_4) :`2` (make `/Game/Levels/STRUCT_Connected_Rooms` _left_4 _right_4 true _down_4) :`3` (make `/Game/Levels/STRUCT_Connected_Rooms` _left_4 _right_4 _up_4 true))) ; Uptade Current Room
                      (`KismetArrayLibrary.Array_Set` (`self.Connected_Rooms`) (`self.Previous_Room`) (select `int` (`self.Main_Loop_Index`) :`0` (make `/Game/Levels/STRUCT_Connected_Rooms` _left_3 true _up_3 _down_3) :`1` (make `/Game/Levels/STRUCT_Connected_Rooms` true _right_3 _up_3 _down_3) :`2` (make `/Game/Levels/STRUCT_Connected_Rooms` _left_3 _right_3 _up_3 true) :`3` (make `/Game/Levels/STRUCT_Connected_Rooms` _left_3 _right_3 true _down_3))) ; Update COnnected Room
                      (goto _label_6)))))
              (:`Try Again`
                (if (< (`self.Extra_Connectrions_Attempts`) 32)
                  (`KismetArrayLibrary.Array_Clear` (`self.Movement_Direrctions`))
                  (set `self.Move_Options` 0)
                  (goto _label_7)
                  (else
                    (`KismetSystemLibrary.PrintString` "ERROR:Cannot add more connections to rooms.")
                    (`KismetArrayLibrary.Array_Clear` (`self.Movement_Direrctions`))
                    (set `self.Move_Options` 0)
                    (break)))))))))
    (:`then_2`
      (for _array_element_5 (`self.Steps_Taken`)
        (set `self.Main_Loop_Index` _array_element_5)
        (bind (_x_coord _y_coord) (`self.1D_Array_To_2D_Coords` (`KismetMathLibrary.Conv_IntToDouble` (`self.Main_Loop_Index`)) (`KismetMathLibrary.Conv_IntToDouble` (`self.Level_Dimensions_X`))))
        (set `self.Position_Current_Room` (`KismetMathLibrary.MakeVector` (* _x_coord _x_2) (* _y_coord _y_2)))
        (switch `int` (+ (`KismetMathLibrary.Conv_BoolToInt` _left_5) (`KismetMathLibrary.Conv_BoolToInt` _right_5) (`KismetMathLibrary.Conv_BoolToInt` _up_5) (`KismetMathLibrary.Conv_BoolToInt` _down_5))
          (:`1`
            (if _left_6
              (set `self.Room_Rotation` 90.0 :!label _label_9)
              (elif _right_6
                (set `self.Room_Rotation` 270.0)
                (elif _up_6
                  (set `self.Room_Rotation` 180.0)
                  (elif _down_6
                    (set `self.Room_Rotation` 0.0)
                    (else
                      (goto _label_9))))))
            (bind _returnvalue_7 (`|SpawnActorFromClass` "/Game/Levels/Generated/Levels/BP_Level_1_connections.BP_Level_1_connections_C" (`KismetMathLibrary.MakeTransform` (+ (`self.Position_Current_Room`) (`self.Starting_Position`)) (`KismetMathLibrary.MakeRotator` 0.0 0.0 (`self.Room_Rotation`))) "Undefined" "OverrideRootScale" null null))
            (bind _asbp_level_1_connections (cast `/Game/Levels/Generated/Levels/BP_Level_1_connections` _returnvalue_7))
            (`KismetArrayLibrary.Array_Set` (`self.Rooms`) (`self.Main_Loop_Index`) _asbp_level_1_connections))
          (:`4`
            (set `self.Room_Rotation` (select `int` (`KismetMathLibrary.RandomInteger` 4) :`0` 0.0 :`1` 90.0 :`2` 180.0 :`3` 270.0 :!type "Float (single-precision)"))
            (bind _returnvalue_8 (`|SpawnActorFromClass` "/Game/Levels/Generated/Levels/BP_Level_4_connections.BP_Level_4_connections_C" (`KismetMathLibrary.MakeTransform` (+ (`self.Position_Current_Room`) (`self.Starting_Position`)) (`KismetMathLibrary.MakeRotator` 0.0 0.0 (`self.Room_Rotation`))) "Undefined" "OverrideRootScale" null null))
            (`KismetArrayLibrary.Array_Set` (`self.Rooms`) (`self.Main_Loop_Index`) _returnvalue_8)))))
    (:`then_3`
      (`KismetSystemLibrary.ExecuteConsoleCommand` "RebuildNavigation" null))))

(fn `1D_Array_To_2D_Coords`
  (params (`1D Array` :type "Float (double-precision)") (`X Dimension` :type "Float (double-precision)"))
  (returns (`X Coord` :type Integer) (`Y Coord` :type Integer))
  (bind _returnvalue (`KismetMathLibrary.FFloor` (/ `1D Array` `X Dimension`)))
  (return (`KismetMathLibrary.FFloor` (- `1D Array` (* _returnvalue `X Dimension`))) _returnvalue))

(fn `UserConstructionScript`)